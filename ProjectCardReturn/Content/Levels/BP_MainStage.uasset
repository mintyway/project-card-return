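; Main stage Blueprint that plays the ending cinematic after Pattern 2 of the Serin doll head succeeds.
; On BeginPlay it binds to the Serin spawn event, then hooks the doll head's Pattern 2 success delegate once that event fires.
; Success plays the LS_End Level Sequence, disabling input and hiding the HUD on the cached Erica character until the sequence finishes.
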(event `self.ReceiveBeginPlay`
  (add `self.OnSpawnSerin` (delegate `OnSpawnSerin_Event`)))

(event `OnSpawnSerin_Event`
  (add `PCRSerinDollHeadCharacter.OnPattern2Succeed` (`self.SerinDollHead`) (delegate `OnPattern2Succeed_이벤트`)))

(event `OnPattern2Succeed_이벤트`
  (bind _cachedericacharacter (`self.CachedEricaCharacter`))
  (bind (_outactor _returnvalue) (`LevelSequencePlayer.CreateLevelSequencePlayer` "/Game/Levels/Sequences/LS_End.LS_End" (make `MovieSceneSequencePlaybackSettings` false (struct) 1.0 0.0 false false true true true true)))
  (add `MovieSceneSequencePlayer.OnFinished` _returnvalue (delegate `OnFinished_이벤트`))
  (`MovieSceneSequencePlayer.Play` _returnvalue)
  (`PCREricaCharacter.SetInput` _cachedericacharacter false)
  (`PCREricaCharacter.SetHUDVisibility` _cachedericacharacter false))

(event `OnFinished_이벤트`
  (bind _cachedericacharacter (`self.CachedEricaCharacter`))
  (`PCREricaCharacter.SetInput` _cachedericacharacter true)
  (`PCREricaCharacter.SetHUDVisibility` _cachedericacharacter true))

(fn `UserConstructionScript`)