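; Main stage Blueprint that scripts the tutorial intro, boss entry and ending cinematics.
; On BeginPlay, chained timers and delegates drive game-mode camera shots of the rabbit and tutorial lights, then call StageStart.
; PlayBossEntryLevelSequence plays the boss intro; once Serin spawns, SerinDollHead's Pattern 2 success triggers the ending sequence.
; Both sequences disable Erica's input and HUD while playing and restore them on finish.
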(event `OnFinished_이벤트_0`
  (bind _cachedericacharacter (`self.CachedEricaCharacter`))
  (`PCREricaCharacter.SetInput` _cachedericacharacter true)
  (`PCREricaCharacter.SetHUDVisibility` _cachedericacharacter true))

(event `커스텀이벤트`
  (`KismetSystemLibrary.K2_SetTimerDelegate` (delegate `커스텀이벤트_4`) 0.5))

(event `self.ReceiveBeginPlay`
  (add `self.OnSpawnSerin` (delegate `OnSpawnSerin_Event`))
  (bind (_outactor _returnvalue) (`LevelSequencePlayer.CreateLevelSequencePlayer` "/Game/Levels/Sequences/LS_BossEntry.LS_BossEntry" (make `MovieSceneSequencePlaybackSettings` false (struct) 1.0 0.0 false false true true true true)))
  (bind _output_get (set `self.BossEntryLevelSequence` _returnvalue))
  (add `MovieSceneSequencePlayer.OnFinished` _output_get (delegate `OnFinished_이벤트_0`))
  (bind _aspcrgame_mode_base (cast `PCRGameModeBase` (`GameplayStatics.GetGameMode`)))
  (bind _outactors (`GameplayStatics.GetAllActorsOfClassWithTag` "/Script/Engine.CameraActor" "ZoomInRabbitCamera"))
  (`self.ZoomInRabbit` _aspcrgame_mode_base (`|GetArrayItem` _outactors))
  (`KismetSystemLibrary.K2_SetTimerDelegate` (delegate `커스텀이벤트`) 5.0)
  (bind _outactors_2 (`GameplayStatics.GetAllActorsOfClassWithTag` "/Script/Engine.CameraActor" "LightOnCamera"))
  (add `PCRTutoRabbit.OnAnimationEnd` (`self.TutoRabbit`) (delegate `OnAnimationEnd_이벤트`)))

(event `커스텀이벤트_4`
  (`self.ZoomOutRabbit` (stale `self.ReceiveBeginPlay` _aspcrgame_mode_base)))

(event `OnAnimationEnd_이벤트`
  (`KismetSystemLibrary.K2_SetTimerDelegate` (delegate `커스텀이벤트_0`) 0.8))

(event `OnSpawnSerin_Event`
  (add `PCRSerinDollHeadCharacter.OnPattern2Succeed` (`self.SerinDollHead`) (delegate `OnPattern2Succeed_이벤트`))
  (bind (_outactor _returnvalue) (`LevelSequencePlayer.CreateLevelSequencePlayer` "/Game/Levels/Sequences/LS_End.LS_End" (make `MovieSceneSequencePlaybackSettings` false (struct) 1.0 0.0 false false true true true true)))
  (bind _output_get (set `self.EndingLevelSequence` _returnvalue))
  (add `MovieSceneSequencePlayer.OnFinished` _output_get (delegate `OnFinished_이벤트`)))

(event `커스텀이벤트_0`
  (`PCRTutorialLight.TurnOnLights` (`self.TutorialLight`))
  (`KismetSystemLibrary.K2_SetTimerDelegate` (delegate `커스텀이벤트_1`) 1.0)
  (`FMODBlueprintStatics.PlayEvent2D` "/Game/FMOD/Events/SFX/Stage/Tutorial_Light.Tutorial_Light"))

(event `OnPattern2Succeed_이벤트`
  (bind _cachedericacharacter (`self.CachedEricaCharacter`))
  (bind _endinglevelsequence (`self.EndingLevelSequence`)
    (:`then`
      (`MovieSceneSequencePlayer.Play` _endinglevelsequence)
      (`PCREricaCharacter.SetInput` _cachedericacharacter false)
      (`PCREricaCharacter.SetHUDVisibility` _cachedericacharacter false))
    (:`else`)))

(event `OnFinished_이벤트`
  (bind _cachedericacharacter (`self.CachedEricaCharacter`))
  (`PCREricaCharacter.SetInput` _cachedericacharacter true)
  (`PCREricaCharacter.SetHUDVisibility` _cachedericacharacter true))

(event `커스텀이벤트_1`
  (`self.StartLightCamera` (stale `self.ReceiveBeginPlay` _aspcrgame_mode_base) (`|GetArrayItem` (stale `self.ReceiveBeginPlay` _outactors_2)))
  (add `PCRTutorialLight.OnLightEnd` (`self.TutorialLight`) (delegate `OnLightEnd_이벤트`)))

(event `OnLightEnd_이벤트`
  (`KismetSystemLibrary.K2_SetTimerDelegate` (delegate `커스텀이벤트_2`) 2.0))

(event `커스텀이벤트_2`
  (`self.EndLightCamera` (stale `self.ReceiveBeginPlay` _aspcrgame_mode_base))
  (`KismetSystemLibrary.K2_SetTimerDelegate` (delegate `커스텀이벤트_3`) 4.0))

(event `커스텀이벤트_3`
  (`self.StageStart`))

(fn `PlayBossEntryLevelSequence`
  (bind _cachedericacharacter (`self.CachedEricaCharacter`))
  (bind _bossentrylevelsequence (`self.BossEntryLevelSequence`)
    (:`then`
      (`MovieSceneSequencePlayer.Play` _bossentrylevelsequence)
      (`PCREricaCharacter.SetInput` _cachedericacharacter false)
      (`PCREricaCharacter.SetHUDVisibility` _cachedericacharacter false))
    (:`else`)))

(fn `UserConstructionScript`)