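; BP_PCRLineMovePanelActor is a panel actor that moves along the spline of a referenced Spline actor.
; MoveTimeline converts an incoming timeline alpha into a distance along the spline length, then sets the world location from it.
; Rotation takes roll and yaw from the spline in local space, with yaw offset by -90 degrees, and keeps the current pitch.
; The event graph is empty, so the alpha must be supplied from outside.
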(event `self.ReceiveBeginPlay`)

(fn `MoveTimeline`
  (params (TimeLineAlpha :type "Float (double-precision)"))
  (bind _spline (`/Game/BlueprintClasses/BP_PCRSpline.Spline` (`self.Spline`)))
  (bind _returnvalue (`KismetMathLibrary.Lerp` 0.0 (`SplineComponent.GetSplineLength` (`/Game/BlueprintClasses/BP_PCRSpline.Spline` (`self.Spline`))) TimeLineAlpha))
  (`self.K2_SetActorLocationAndRotation` (`SplineComponent.GetLocationAtDistanceAlongSpline` _spline _returnvalue "World") (`KismetMathLibrary.MakeRotator` (.roll (`SplineComponent.GetRotationAtDistanceAlongSpline` _spline _returnvalue "Local")) (.pitch (`self.K2_GetActorRotation`)) (+ (.yaw (`SplineComponent.GetRotationAtDistanceAlongSpline` _spline _returnvalue "Local")) -90.0))))

(fn `UserConstructionScript`)