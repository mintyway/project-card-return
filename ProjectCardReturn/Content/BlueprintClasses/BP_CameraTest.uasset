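; BP_CameraTest is a test actor that briefly switches the player's view to a fixed camera when an actor overlaps it.
; On overlap, it gets the player controller through the game mode's cached Erica character and sets the view target to the first CameraActor tagged "CameraTest".
; A one-shot timer then fires a custom event that blends the view back to Erica after a few seconds.
; The overlapping actor is not checked.
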(event `self.ReceiveActorBeginOverlap`
  (params (OtherActor :type "Actor Object Reference"))
  (bind _aspcrgame_mode_base (cast `PCRGameModeBase` (`GameplayStatics.GetGameMode`)))
  (bind `_as플레이어_컨트롤러` (cast `PlayerController` (`Pawn.GetController` (`PCRGameModeBase.CachedEricaCharacter` _aspcrgame_mode_base))))
  (bind _outactors (`GameplayStatics.GetAllActorsOfClassWithTag` "/Script/Engine.CameraActor" "CameraTest"))
  (`PlayerController.SetViewTargetWithBlend` `_as플레이어_컨트롤러` (`|GetArrayItem` _outactors) 0.0 "VTBlend_Linear" 0.0 false)
  (`KismetSystemLibrary.K2_SetTimerDelegate` (delegate `커스텀이벤트`) 3.0))

(event `커스텀이벤트`
  (`PlayerController.SetViewTargetWithBlend` (stale `self.ReceiveActorBeginOverlap` `_as플레이어_컨트롤러`) (`PCRGameModeBase.CachedEricaCharacter` (stale `self.ReceiveActorBeginOverlap` _aspcrgame_mode_base)) 1.0 "VTBlend_Linear" 0.0 false))

(fn `UserConstructionScript`)