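; BP_PCRBossEntryZone is a one-shot trigger zone that starts the boss entry cinematic after Stage 1.
; Collision is off until the game mode's OnStage1End event enables it and shows the player HUD.
; An overlap, with no check on the other actor, plays the main stage's boss entry Level Sequence and moves Erica to the zone's XY at her current height.
; It then hides the HUD and Stage 1 UI and destroys itself.
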(event `self.ReceiveBeginPlay`
  (`self.SetActorEnableCollision` false)
  (bind _aspcrgame_mode_base (cast `PCRGameModeBase` (`GameplayStatics.GetGameMode`)))
  (add `PCRGameModeBase.OnStage1End` _aspcrgame_mode_base (delegate `OnStage1End_이벤트`)))

(event `OnStage1End_이벤트`
  (`self.SetActorEnableCollision` true)
  (bind _aspcrerica_player_controller (cast `PCREricaPlayerController` (`GameplayStatics.GetPlayerController` 0)))
  (`PCREricaPlayerController.SetVisibilityHUD` _aspcrerica_player_controller true))

(event `self.ReceiveActorBeginOverlap`
  (params (OtherActor :type "Actor Object Reference"))
  (bind _asbp_pcrmain_stage (cast `/Game/BlueprintClasses/BP_PCRMainStage` (`GameplayStatics.GetGameMode`)))
  (`/Game/BlueprintClasses/BP_PCRMainStage.PlayBossEntryLevelSequence` _asbp_pcrmain_stage)
  (`self.K2_SetActorLocation` (`PCRGameModeBase.CachedEricaCharacter` _asbp_pcrmain_stage) (`KismetMathLibrary.MakeVector` (.x (`self.K2_GetActorLocation`)) (.y (`self.K2_GetActorLocation`)) (.z (`self.K2_GetActorLocation` (`PCRGameModeBase.CachedEricaCharacter` _asbp_pcrmain_stage)))) false false)
  (bind _aspcrerica_player_controller (cast `PCREricaPlayerController` (`GameplayStatics.GetPlayerController` 0)))
  (`PCREricaPlayerController.SetVisibilityHUD` _aspcrerica_player_controller false)
  (`PCREricaPlayerController.SetVisibilityStage1UI` _aspcrerica_player_controller false)
  (`self.K2_DestroyActor`))

(fn `UserConstructionScript`)