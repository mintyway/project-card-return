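; BP_CatPanel is a movable environment panel that starts moving automatically shortly after play begins.
; BeginPlay runs the parent logic, then sets a one-shot two-second timer that fires a custom event to play a timeline.
; Each timeline update passes its Alpha to MoveTimeline, whose movement logic is defined outside this graph.
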(event `self.ReceiveBeginPlay`
  (`parent.ReceiveBeginPlay`)
  (`KismetSystemLibrary.K2_SetTimerDelegate` (delegate `커스텀이벤트`) 2.0))

(event `커스텀이벤트`
  (bind (_direction _alpha) (`Timeline|타임라인`)
    (:`Update`
      (`self.MoveTimeline` _alpha))))

(fn `UserConstructionScript`
  (`parent.UserConstructionScript`))