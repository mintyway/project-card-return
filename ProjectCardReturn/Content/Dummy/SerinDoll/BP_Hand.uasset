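; BP_Hand is a character Blueprint for the Serin Doll's left hand that repeats an attack animation on a timer.
; On BeginPlay it assigns the left-hand AnimBlueprint to the mesh, turns off gravity and starts a looping timer that calls PlayAttack by name.
; PlayAttack plays the hand montage on the anim instance and writes a debug log message; the file contains no hit or damage logic.
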(event `self.ReceiveBeginPlay`
  (bind _mesh (`self.Mesh`))
  (`SkeletalMeshComponent.SetAnimationMode` _mesh "AnimationBlueprint" true)
  (`SkeletalMeshComponent.SetAnimInstanceClass` _mesh "/Game/Dummy/SerinDoll/SK_SerinDoll_LeftHand_Skeleton2_AnimBlueprint2.SK_SerinDoll_LeftHand_Skeleton2_AnimBlueprint2_C")
  (set `CharacterMovementComponent.GravityScale` 0.0 (`self.CharacterMovement`))
  (`KismetSystemLibrary.K2_SetTimer` null "PlayAttack" 5.0 true))

(event `self.ReceiveTick`
  (params (DeltaSeconds :type "Float (single-precision)")))

(fn `PlayAttack`
  (`AnimInstance.Montage_Play` (`SkeletalMeshComponent.GetAnimInstance` (`self.Mesh`)) "/Game/Dummy/SerinDoll/SK_SerinDoll_LeftHand_Skeleton2_Montage2.SK_SerinDoll_LeftHand_Skeleton2_Montage2" 1.0 "MontageLength" 0.0 true)
  (`KismetSystemLibrary.LogString` "Hello"))

(fn `UserConstructionScript`)