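; BP_MainStage is a main stage Blueprint that triggers the ending cinematic of the Serin encounter.
; When Serin spawns, it creates a non-autoplay player for LS_End and binds to SerinDollHead's Pattern 2 success event.
; That success plays the sequence while disabling Erica's input and hiding her HUD, both restored when the sequence finishes.
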(event `self.ReceiveBeginPlay`
  (add `self.OnSpawnSerin` (delegate `OnSpawnSerin_Event`)))

(event `OnSpawnSerin_Event`
  (add `PCRSerinDollHeadCharacter.OnPattern2Succeed` (`self.SerinDollHead`) (delegate `OnPattern2Succeed_이벤트`))
  (bind (_outactor _returnvalue) (`LevelSequencePlayer.CreateLevelSequencePlayer` "/Game/Levels/Sequences/LS_End.LS_End" (make `MovieSceneSequencePlaybackSettings` false (struct) 1.0 0.0 false false true true true true)))
  (bind _output_get (set `self.EndingLevelSequence` _returnvalue))
  (add `MovieSceneSequencePlayer.OnFinished` _output_get (delegate `OnFinished_이벤트`)))

(event `OnPattern2Succeed_이벤트`
  (bind _cachedericacharacter (`self.CachedEricaCharacter`))
  (bind _endinglevelsequence (`self.EndingLevelSequence`)
    (:`then`
      (`MovieSceneSequencePlayer.Play` _endinglevelsequence)
      (`PCREricaCharacter.SetInput` _cachedericacharacter false)
      (`PCREricaCharacter.SetHUDVisibility` _cachedericacharacter false))
    (:`else`)))

(event `OnFinished_이벤트`
  (bind _cachedericacharacter (`self.CachedEricaCharacter`))
  (`PCREricaCharacter.SetInput` _cachedericacharacter true)
  (`PCREricaCharacter.SetHUDVisibility` _cachedericacharacter true))

(fn `UserConstructionScript`)