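; BP_LineMoveActor is an actor that moves along the path of a referenced spline.
; On BeginPlay, if the Spline reference is valid, it plays a timeline whose track maps onto the spline's length as a distance.
; Each update sets the actor's location and rotation at that distance.
; Location is sampled in world space but rotation in local space, so the spline's own rotation is not applied to the actor's orientation.
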(event `self.ReceiveBeginPlay`
  (bind _spline (`/Game/Blueprints/BP_Spline.Spline` (`self.Spline`)))
  (`self.Spline`
    (:`then`
      (bind (_direction `_새_트랙_0`) (`Timeline|타임라인`)
        (:`Update`
          (bind _returnvalue (`KismetMathLibrary.Lerp` 0.0 (`SplineComponent.GetSplineLength` (`/Game/Blueprints/BP_Spline.Spline` (`self.Spline`))) `_새_트랙_0`))
          (`self.K2_SetActorLocationAndRotation` (`SplineComponent.GetLocationAtDistanceAlongSpline` _spline _returnvalue "World") (`SplineComponent.GetRotationAtDistanceAlongSpline` _spline _returnvalue "Local")))))
    (:`else`)))

(fn `UserConstructionScript`)